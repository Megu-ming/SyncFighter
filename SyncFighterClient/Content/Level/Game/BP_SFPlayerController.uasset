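; Player controller that owns the on-screen menu and chat widgets and handles their hotkeys.
; On BeginPlay it creates both widgets and adds them to the viewport, with the menu starting hidden.
; Escape toggles the menu's visibility, switching between UI-only and game-only input and showing or hiding the mouse cursor.
; Enter forwards to the chat widget's OnChat.
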(event EventBeginPlay
  (bind _returnvalue (UserInterface|CreateWidget "/Game/UI/GameUI/WBP_Menu.WBP_Menu_C"))
  (Variables|Default|SetMenuWidget _returnvalue)
  (UserInterface|Viewport|AddtoViewport (Variables|Default|GetMenuWidget) 0)
  (Widget|SetVisibility (Variables|Default|GetMenuWidget) "Hidden")
  (bind _returnvalue_2 (UserInterface|CreateWidget "/Game/UI/GameUI/WBP_Chat.WBP_Chat_C"))
  (bind _output_get (Variables|Default|SetChatWidget _returnvalue_2))
  (UserInterface|Viewport|AddtoViewport _output_get 0))

(event Input|KeyboardEvents|Escape
  (params (Key :type Key%20Structure :default "None"))
  (bind _menuwidget (Variables|Default|GetMenuWidget))
  (:Pressed
    (if (Widget|IsVisible (Variables|Default|GetMenuWidget))
      (Widget|SetVisibility _menuwidget "Hidden")
      (Input|SetInputModeGameOnly 0 false)
      (Variables|Default|SetbShowMouseCursor false)
      (else
        (Widget|SetVisibility _menuwidget "Visible")
        (Input|SetInputModeUIOnly 0 (Variables|Default|GetMenuWidget) "DoNotLock" false)
        (Variables|Default|SetbShowMouseCursor true)))))

(event Input|KeyboardEvents|Enter
  (params (Key :type Key%20Structure :default "None"))
  (:Pressed
    (Class|SFChatWidget|OnChat (Variables|Default|GetChatWidget))))

(fn ConstructionScript)