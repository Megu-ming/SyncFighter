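; BP_CosmicRift is a Mage skill actor that deals area damage to characters around its location, ignoring the instigator.
; After a short delay it applies a heavy initial hit, then a looping timer runs ApplyMeteorShower for lighter repeat hits over two seconds.
; Only the locally controlled instigator runs the sphere overlaps, reporting damage through SFGameInstance's SendHitReq by PlayerID.
; The timed cleanup and self-destroy also run only on that client.
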(event Custom|ApplyMeteorShower
  (bind _returnvalue (Game|GetInstigator))
  (if (Pawn|IsLocallyControlled _returnvalue)
    (bind _outactors (Collision|SphereOverlapActors (Transformation|GetActorLocation) 3e+02 (Variables|Default|GetObject%20Types) 0 (Utilities|Array|MakeArray _returnvalue)))
    (for _array_element _outactors
      (bind _assfcharacter (Utilities|Casting|CastToSFCharacter _array_element))
      (bind _assfgame_instance (Utilities|Casting|CastToSFGameInstance (Game|GetGameInstance)))
      (Class|SFGameInstance|SendHitReq _assfgame_instance (Variables|/Script/SyncFighterClient.SFCharacter|GetPlayerID _assfcharacter) 10))))

(event EventBeginPlay
  (bind _returnvalue (Game|GetInstigator))
  (Utilities|FlowControl|Delay 0.5)
  (Utilities|IsValid _returnvalue
    (:Is%20Valid
      (if (Pawn|IsLocallyControlled _returnvalue)
        (bind _outactors (Collision|SphereOverlapActors (Transformation|GetActorLocation) 3e+02 (Variables|Default|GetObject%20Types) 0 (Utilities|Array|MakeArray _returnvalue)))
        (for _array_element _outactors
          (bind _assfcharacter (Utilities|Casting|CastToSFCharacter _array_element))
          (bind _assfgame_instance (Utilities|Casting|CastToSFGameInstance (Game|GetGameInstance)))
          (Class|SFGameInstance|SendHitReq _assfgame_instance (Variables|/Script/SyncFighterClient.SFCharacter|GetPlayerID _assfcharacter) 40))
        (bind _returnvalue_2 (Utilities|Time|SetTimerbyEvent (delegate Custom|ApplyMeteorShower) 0.6 true))
        (Variables|Default|SetShowerTimerHandle _returnvalue_2)
        (Utilities|FlowControl|Delay 2.0)
        (Utilities|Time|ClearandInvalidateTimerbyHandle (Variables|Default|GetShowerTimerHandle))
        (Utilities|FlowControl|Delay 1.0)
        (Actor|DestroyActor)))))

(fn ConstructionScript)